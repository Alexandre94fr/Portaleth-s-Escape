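; BP_Lever is an interactable lever that toggles a linked BP_Door between rest and activated rotations.
; On BeginPlay it applies the same indicator material to itself and the door, visually pairing them.
; Player interaction flips IsLeverActivated, then InteractWithDoor calls Interact to rotate the door and sets the handle rotation instantly.
; A sphere trigger shows or hides an optional tip widget on overlap.
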(event `self.ReceiveBeginPlay`
  (bind _indictormaterial (`self.IndictorMaterial`))
  (`PrimitiveComponent.SetMaterial` (`self.Indicator`) 0 _indictormaterial)
  (bind _asbp_door (cast `/Game/Interactables/Door/BP_Door` (`self.LinkedDoor`))
    (:`then`
      (`PrimitiveComponent.SetMaterial` (`/Game/Interactables/Door/BP_Door.Indicator` _asbp_door) 0 _indictormaterial))
    (:`CastFailed`
      (`KismetSystemLibrary.PrintString` "ERROR ! Cast failed, check if you give LinkedDoor variable a value. " true true (struct :`R` 1.0 :`A` 1.0) 5.0))))

(event `/Game/Interactables/BPI_Interactable.GetInteractedByPlayer`
  (bind _linkeddoor (`self.LinkedDoor`))
  (bind _handlerotationroot (`self.HandleRotationRoot`))
  (if (`self.isLeverActivated`)
    (set `self.isLeverActivated` false)
    (`self.InteractWithDoor` _linkeddoor _handlerotationroot)
    (else
      (set `self.isLeverActivated` true)
      (`self.InteractWithDoor` _linkeddoor _handlerotationroot (`self.LeverNewRotationWhenActivated`)))))

(event `self.ActionTriggererSphereCollider.OnComponentBeginOverlap`
  (params (OverlappedComponent :type "PrimitiveComponent Object Reference") (OtherActor :type "Actor Object Reference") (OtherComp :type "PrimitiveComponent Object Reference") (OtherBodyIndex :type Integer) (bFromSweep :type Boolean) (SweepResult :type "HitResult Structure (by ref)"))
  (set `self.isInRange` true)
  (if (`self.IsTipsEnable`)
    (`SceneComponent.SetVisibility` (`self.TipsWidget`) true false)))

(event `self.ActionTriggererSphereCollider.OnComponentEndOverlap`
  (params (OverlappedComponent :type "PrimitiveComponent Object Reference") (OtherActor :type "Actor Object Reference") (OtherComp :type "PrimitiveComponent Object Reference") (OtherBodyIndex :type Integer))
  (if (`self.IsTipsEnable`)
    (`SceneComponent.SetVisibility` (`self.TipsWidget`) false false)))

(event `/Game/Interactables/BPI_Interactable.Interact`
  (params (InteractedObject :type "Actor Object Reference"))
  (bind _asbp_door (cast `/Game/Interactables/Door/BP_Door` InteractedObject)
    (:`then`
      (if (`self.isLeverActivated`)
        (bind _doorrotationroot (`/Game/Interactables/Door/BP_Door.DoorRotationRoot` _asbp_door))
        (`SceneComponent.K2_SetRelativeRotation` _doorrotationroot (`self.DoorNewRotationWhenActivated`) false false)
        (else
          (`SceneComponent.K2_SetRelativeRotation` :`self` _doorrotationroot))))
    (:`CastFailed`
      (`KismetSystemLibrary.PrintString` "ERROR ! Cast failed, check if you give LinkedDoor variable a value. " true true (struct :`R` 1.0 :`A` 1.0) 5.0))))

(fn `UserConstructionScript`)